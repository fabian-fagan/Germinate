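; Castle parallax background actor that follows a character and animates a day-night cycle on a dynamic material plane.
; A Timeline, with adjustable play rate and start time, drives sky, mountain, cloud, sun, moon and window-glow colors each update.
; The same update scrolls layers at divided rates from character X, drifts clouds and stars by velocity, and rotates sun and moon by time.
; A lagging spring arm keeps the backdrop positioned at the character.
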(event EventBeginPlay
  (|CreateMaterialIns)
  (Components|Timeline|SetPlayRate (Variables|Default|GetTimeline) (Variables|Default|GetPlayRate))
  (Components|Timeline|SetNewTime (Variables|Default|GetTimeline) (Variables|Default|GetSetTime))
  (bind (_direction _time _starsbrightness _glowplacement _topsky _bottomsky _bottomskyleft _bottomskyright _overallcolorandbrightness _backmountain _middlemountain _frontmountain _clouds _mooncolor _suncolor _windowglow) (Timeline|Timeline Play)
    (:Update
      (|SkyColors _starsbrightness _glowplacement _topsky _bottomsky _bottomskyleft _bottomskyright _overallcolorandbrightness _backmountain _middlemountain _frontmountain _clouds _mooncolor _suncolor _windowglow)
      (|TimelineUpdateParallaxOffset)
      (|SetTimerAndRotator _time)
      (|CloudSpeed)
      (|SunAndMoonPosition)
      (|CharacterPosition)
      (CallFunction|UpdateParallaxScrolling (Variables|Default|GetParallaxOffset)))))

(fn ConstructionScript)

(fn UpdateParallaxScrolling
  (params (NewOffset :type Float%20%28single-precision%29))
  (bind _movingbasedonspeed (Variables|Default|GetMovingBasedOnSpeed))
  (Rendering|Material|SetScalarParameterValueonMaterials (Variables|Default|GetPlane) "OffsetLayer0" (/ NewOffset 4.0))
  (Rendering|Material|SetScalarParameterValueonMaterials (Variables|Default|GetPlane) "OffsetLayer1" (/ NewOffset 2.0))
  (Rendering|Material|SetScalarParameterValueonMaterials (Variables|Default|GetPlane) "OffsetLayer2" NewOffset)
  (Rendering|Material|SetScalarParameterValueonMaterials (Variables|Default|GetPlane) "OffsetStars" (/ _movingbasedonspeed 32.0))
  (Rendering|Material|SetScalarParameterValueonMaterials (Variables|Default|GetPlane) "OffsetClouds" (/ _movingbasedonspeed 16.0))
  (Rendering|Material|SetScalarParameterValueonMaterials (Variables|Default|GetPlane) "OffsetCloudsFront" (/ _movingbasedonspeed 4.0)))